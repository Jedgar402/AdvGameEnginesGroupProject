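; BP_PlayerCharacter is the player character Blueprint, which displays its health through an on-screen UI widget.
; On BeginPlay it creates WB_UI, stores the reference, adds it to the viewport and sends it the current and maximum values from Health.
; AnyDamage pushes the same values to the widget again, with no health calculation in this graph.
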(event EventBeginPlay
  (bind _health (Variables|Default|GetHealth))
  (bind _returnvalue (UserInterface|CreateWidget "/Game/WB_UI.WB_UI_C"))
  (bind _output_get (Variables|Default|SetUI%20Ref _returnvalue))
  (UserInterface|Viewport|AddtoViewport _output_get 0)
  (Default|UpdateHealth (Variables|Default|GetUI%20Ref) (Variables|/Script/GroupProject_FPS.HealthComponent|GetHealth _health) (Variables|/Script/GroupProject_FPS.HealthComponent|GetMaxHealth _health)))

(event Game|Damage|EventAnyDamage
  (params (Damage :type Float%20%28single-precision%29) (DamageType :type Damage%20Type%20Object%20Reference) (InstigatedBy :type Controller%20Object%20Reference) (DamageCauser :type Actor%20Object%20Reference))
  (bind _health (Variables|Default|GetHealth))
  (Default|UpdateHealth (Variables|Default|GetUI%20Ref) (Variables|/Script/GroupProject_FPS.HealthComponent|GetHealth _health) (Variables|/Script/GroupProject_FPS.HealthComponent|GetMaxHealth _health)))

(fn ConstructionScript)